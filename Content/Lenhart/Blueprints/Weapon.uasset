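; Weapon Blueprint that fires projectiles automatically while its trigger is held.
; PullTrigger passes through a DoOnce gate, fires immediately, then starts a looping timer on Fire at an interval derived from RPS.
; ReleaseTrigger clears the timer and resets the gate.
; Each Fire call spawns the Projectile class at the ProjectileSpawnPoint transform.
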(event Custom|PullTrigger
  ;[1 1 1] Pulling the Trigger
  (Utilities|FlowControl|DoOnce false
    (:Completed
      (CallFunction|Fire)
      (Utilities|Time|SetTimerbyFunctionName 0 "Fire" (/ 1.0 (Variables|Default|GetRPS)) true))))

(event Custom|ReleaseTrigger
  (Utilities|Time|ClearTimerbyFunctionName 0 "Fire")
  ;[1 1 1] Pulling the Trigger
  (Utilities|FlowControl|DoOnce false) ; enters at Reset
)

(event Custom|Fire
  ;[1 1 1] Firing Mech
  (Game|SpawnActorfromClass "/Game/Lenhart/Blueprints/Projectile.Projectile_C" (Transformation|GetWorldTransform (Variables|Default|GetProjectileSpawnPoint)) "Undefined" 0 0))

(fn ConstructionScript)